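; BP_P38 is a player-controlled P-38 plane pawn that constantly flies forward and fires rockets.
; Tick feeds forward movement input, intended for FloatingPawnMovement, and spins the left and right propellers through RotatePropeller.
; Enhanced Input applies frame-rate-scaled local roll and pitch, and spawns BP_Rocket at the Arrow component's transform.
; Legacy axis events are empty, and hand-written movement and rotation nodes remain disconnected.
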(event Input|EnhancedActionEvents|EnhancedInputActionIA_Fire
  (params (ActionValue :type Boolean) (ElapsedSeconds :type Float%20%28double-precision%29) (TriggeredSeconds :type Float%20%28double-precision%29) (InputAction :type Input%20Action%20Object%20Reference :default "/Game/Blueprints/Input/IA_Fire.IA_Fire"))
  (bind _arrow (Variables|Default|GetArrow))
  ;[0.15 0.15 0.15 0.5] 미사일 발사
  (Game|SpawnActorfromClass "/Game/Blueprints/BP_Rocket.BP_Rocket_C" (Math|Transform|MakeTransform (Transformation|GetWorldLocation _arrow) (Transformation|GetWorldRotation _arrow) "1.000000,1.000000,1.000000") "Undefined" "MultiplyWithRoot" 0 self))

(event Input|EnhancedActionEvents|EnhancedInputActionIA_Movement
  (params (ActionValue :type Vector%202D%20Structure) (ElapsedSeconds :type Float%20%28double-precision%29) (TriggeredSeconds :type Float%20%28double-precision%29) (InputAction :type Input%20Action%20Object%20Reference :default "/Game/Blueprints/Input/IA_Movement.IA_Movement"))
  (:Triggered
    (Transformation|AddActorLocalRotation (Math|Rotator|MakeRotator (* (.x ActionValue) (Utilities|Time|GetWorldDeltaSeconds) 6e+01) 0.0 0.0) false false)
    (Transformation|AddActorLocalRotation (Math|Rotator|MakeRotator 0.0 (* (.y ActionValue) (Utilities|Time|GetWorldDeltaSeconds) 6e+01) 0.0) false false)))

(event EventTick
  (params (DeltaSeconds :type Float%20%28single-precision%29))
  (Utilities|FlowControl|Sequence
    (:then_0
      ;[0.15 0.15 0.15 0.5] FloatingPawnMovement이용
      (Pawn|Input|AddMovementInput (Transformation|GetActorForwardVector) 1.0 false))
    (:then_1
      ;[0.15 0.15 0.15 0.5] 프로펠러 회전
      (CallFunction|RotatePropeller (Variables|Default|GetLeft))
      (CallFunction|RotatePropeller (Variables|Default|GetRight)))))

(event Input|ActionEvents|InputActionFire
  (params (Key :type Key%20Structure :default "None"))
  ;[0.15 0.15 0.15 0.5] 미사일 발사
)

(event Input|AxisEvents|InputAxisPitch
  (params (AxisValue :type Float%20%28single-precision%29))
  ;[0.15 0.15 0.15 0.5] 조종
)

(event Input|AxisEvents|InputAxisRoll
  (params (AxisValue :type Float%20%28single-precision%29))
  ;[0.15 0.15 0.15 0.5] 조종
)

(fn ConstructionScript)

(fn RotatePropeller
  (params (Location :type Scene%20Component%20Object%20Reference))
  (Transformation|AddLocalRotation Location (Math|Rotator|MakeRotator (* (Variables|Default|GetPropellerRotation) (Utilities|Time|GetWorldDeltaSeconds)) 0.0 0.0) false false))